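; VTOL aircraft actor that flies between helipads at a set height, needing control tower clearance for each leg.
; NewDestination sphere-traces toward the destination pad, turning hits into spline points and a tower request queue.
; Approvals trigger liftoff or resume timeline-driven spline movement at constant speed, releasing towers as it advances.
; It records tower waiting times and, after landing, passes them to a Python component to save as text.
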(event `self.ReceiveBeginPlay`
  ;[1 1 1] BeginPlay
  (bind _asmap_base (cast `/Game/MapBase/MapBase` (`GameplayStatics.GetGameMode`)))
  (add `/Game/MapBase/MapBase.InitializeVTOL` _asmap_base (delegate `Initialize`)))

(event `Initialize`
  (bind (_properties_height _properties_speed _properties_destinationtower _properties_destinationpad _properties_destinationpadnum _properties_startingtower _properties_startingpad) (break `/Game/VTOL/VTOL_Properties` (`self.Properties`)))
  ;[1 1 1] BeginPlay
  (`SceneComponent.SetVisibility` (`self.DefaultSceneRoot`) false true)
  (`SceneComponent.SetVisibility` (`self.Spline`) false true)
  (`SceneComponent.SetVisibility` (`self.Beam`) false false)
  (`MeshComponent.SetVectorParameterValueOnMaterials` (`self.SphereOutline`) "Base Color" (`KismetMathLibrary.MakeVector` (`KismetMathLibrary.RandomFloatInRange` 0.0 1.0) (`KismetMathLibrary.RandomFloatInRange` 0.0 1.0) (`KismetMathLibrary.RandomFloatInRange` 0.0 1.0)))
  (`MeshComponent.SetVectorParameterValueOnMaterials` (`self.Ghost_No_Props`) "Base Color" (`KismetMathLibrary.MakeVector` (`KismetMathLibrary.RandomFloatInRange` 0.0 1.0) (`KismetMathLibrary.RandomFloatInRange` 0.0 1.0) (`KismetMathLibrary.RandomFloatInRange` 0.0 1.0)))
  (set `self.Height` _properties_height)
  (`KismetArrayLibrary.Array_AddUnique` (`self.TowerRequest`) (make `/Game/VTOL/VTOL_Struct` false _properties_startingtower))
  (bind _ashelipad_bp (cast `/Game/Objects/Helipad/Helipad_BP` _properties_startingpad))
  (bind _output_get (set `self.PadCoordinates` (`SceneComponent.K2_GetComponentLocation` (`/Game/Objects/Helipad/Helipad_BP.helipad` _ashelipad_bp))))
  (`self.K2_SetActorLocation` _output_get))

(event `self.ReceiveTick`
  (params (DeltaSeconds :type "Float (single-precision)"))
  (bind (_properties_height _properties_speed _properties_destinationtower) (break `/Game/VTOL/VTOL_Properties` (`self.Properties`)))
  (bind (_returnvalue_x _returnvalue_y) (`KismetMathLibrary.BreakVector` (`self.K2_GetActorLocation` _properties_destinationtower)))
  ;[1 1 1] Event Tick
  (`SceneComponent.K2_AddRelativeRotation` (`self.StaticMesh`) (struct :`Yaw` 15.0) false false)
  (`SceneComponent.K2_AddRelativeRotation` (`self.StaticMesh3`) (struct :`Yaw` 15.0) false false)
  (`SceneComponent.K2_AddRelativeRotation` (`self.StaticMesh1`) (struct :`Yaw` -15.0) false false)
  (`SceneComponent.K2_AddRelativeRotation` (`self.StaticMesh2`) (struct :`Yaw` -15.0) false false)
  (`ParticleSystemComponent.SetBeamSourcePoint` (`self.Beam`) 0 (`self.K2_GetActorLocation`) 0)
  (`ParticleSystemComponent.SetBeamTargetPoint` (`self.Beam`) 0 (`KismetMathLibrary.MakeVector` _returnvalue_x _returnvalue_y (`self.Height`)) 0))

(event `NewDestination`
  (bind (_returnvalue_x _returnvalue_y) (`KismetMathLibrary.BreakVector` (`self.K2_GetActorLocation`)))
  (bind _spline (`self.Spline`))
  (bind (_properties_height _properties_speed _properties_destinationtower _properties_destinationpad) (break `/Game/VTOL/VTOL_Properties` (`self.Properties`)))
  ;[1 1 1] NewDestination
  (`SceneComponent.SetVisibility` (`self.DefaultSceneRoot`) true true)
  (`KismetSystemLibrary.Delay` 1.0)
  (`TimelineComponent.Stop` (`self.Drone Movement`))
  (`SplineComponent.ClearSplinePoints` (`self.Spline`) false)
  (`KismetArrayLibrary.Array_Clear` (`self.SplinePoints`))
  (bind _ashelipad_bp (cast `/Game/Objects/Helipad/Helipad_BP` _properties_destinationpad))
  (bind _outactors (`GameplayStatics.GetAllActorsOfClass` "VTOL_BP_C"))
  (bind _helipad (`/Game/Objects/Helipad/Helipad_BP.helipad` _ashelipad_bp))
  (bind (_returnvalue_x_2 _returnvalue_y_2) (`KismetMathLibrary.BreakVector` (`SceneComponent.K2_GetComponentLocation` _helipad)))
  (bind _outhits (`KismetSystemLibrary.SphereTraceMultiForObjects` (`KismetMathLibrary.MakeVector` _returnvalue_x _returnvalue_y (`self.Height`)) (`KismetMathLibrary.MakeVector` _returnvalue_x_2 _returnvalue_y_2 (`self.Height`)) 300.0 (`self.CollisionActor`) false _outactors "None" true (struct :`R` 1.0 :`A` 1.0) (struct :`G` 1.0 :`A` 1.0) 0.0))
  (for _array_element _outhits
    (if (== (`KismetArrayLibrary.Array_Find` (`self.SplinePoints`) (`.Location` (`GameplayStatics.BreakHitResult` _array_element))) -1)
      _
      (else
        _))
    (`KismetArrayLibrary.Array_Add` (`self.SplinePoints`) (`.Location` (`GameplayStatics.BreakHitResult` _array_element)))
    (`SplineComponent.AddSplinePoint` (`self.Spline`) (`.Location` (`GameplayStatics.BreakHitResult` _array_element)) "World" true)
    (`KismetArrayLibrary.Array_AddUnique` (`self.TowerRequest`) (make `/Game/VTOL/VTOL_Struct` false (`.HitActor` (`GameplayStatics.BreakHitResult` _array_element)))))
  (bind (_returnvalue_x_3 _returnvalue_y_3) (`KismetMathLibrary.BreakVector` (`SceneComponent.K2_GetComponentLocation` _helipad)))
  (`SplineComponent.AddSplinePoint` _spline (`KismetMathLibrary.MakeVector` _returnvalue_x_3 _returnvalue_y_3 (`self.Height`)) "World" true)
  (for _index (range (`SplineComponent.GetNumberOfSplinePoints` _spline))
    (`SplineComponent.SetSplinePointType` _spline _index "CurveClamped" true))
  (if (`self.Launching`)
    (`SceneComponent.K2_DetachFromComponent` (`self.Spline`) "KeepWorld" "KeepWorld" "KeepWorld" true)
    (`self.CreateRequest` 0)
    (set `self.Launching` false)
    (else
      (`self.CreateRequest` 0)
      (`self.Move`))))

(event `Liftoff`
  (bind (_padcoordinates_x _padcoordinates_y _padcoordinates_z) (`KismetMathLibrary.BreakVector` (`self.PadCoordinates`)))
  (bind (_output_requested _output_tower _output_approved) (break `/Game/VTOL/VTOL_Struct` (`|GetArrayItem` (`self.TowerRequest`))))
  ;[1 1 1] Liftoff
  (if _output_approved
    (`KismetSystemLibrary.Delay` 0.2)
    (bind (_direction _liftland) (`Timeline|Rise` :!via `PlayFromStart`)
      (:`Update`
        (`self.K2_SetActorLocationAndRotation` (`KismetMathLibrary.MakeVector` _padcoordinates_x _padcoordinates_y (`KismetMathLibrary.Lerp` _padcoordinates_z (`self.Height`) _liftland)) (`KismetMathLibrary.RLerp` (`self.K2_GetActorRotation`) (`SplineComponent.GetRotationAtDistanceAlongSpline` (`self.Spline`) 0.01 "World") (/ _liftland 4.0) true))
        (`SceneComponent.K2_SetRelativeRotation` (`self.Mesh`) (`KismetMathLibrary.MakeRotator` (`KismetMathLibrary.Lerp` 0.0 15.0 _liftland) 0.0 -90.0) false false))
      (:`Finished`
        (`KismetSystemLibrary.Delay` 0.5)
        (`SceneComponent.SetVisibility` (`self.Beam`) true false)
        (set `self.StoppingPoint` 0)
        (`self.Move`)))))

(event `CreateRequest`
  (params (RequestIndex :type Integer))
  (bind _towerrequest (`self.TowerRequest`))
  (bind (_properties_height _properties_speed _properties_destinationtower _properties_destinationpad _properties_destinationpadnum) (break `/Game/VTOL/VTOL_Properties` (`self.Properties`)))
  (bind (_output_requested _output_tower _output_approved) (break `/Game/VTOL/VTOL_Struct` (`|GetArrayItem` _towerrequest RequestIndex)))
  ;[1 1 1] CreateRequest
  (if (> RequestIndex (- (`KismetArrayLibrary.Array_Length` _towerrequest) 1))
    _
    (elif (not _output_requested)
      (`KismetArrayLibrary.Array_Set` _towerrequest RequestIndex (make `/Game/VTOL/VTOL_Struct` true _output_tower _output_approved))
      (if (== _output_tower _properties_destinationtower)
        (set `self.PadNum` _properties_destinationpadnum)
        (else
          (set `self.PadNum` 4)))
      (bind _ascontrol_tower_bp2 (cast `/Game/Objects/ControlTower/ControlTowerBP2` _output_tower))
      (`/Game/Objects/ControlTower/ControlTowerBP2.CreateRequest` _ascontrol_tower_bp2 self (`self.PadNum`))
      (`BlueprintMapLibrary.Map_Add` (`self.Time`) "Start" (`GameplayStatics.GetTimeSeconds`)))))

(event `Resume`
  (bind _spline (`self.Spline`))
  (bind _spline_2 (`self.Spline`))
  (bind _stoppingpoint (`self.StoppingPoint`))
  (bind _stoppingpoint_2 (`self.StoppingPoint`))
  (bind _returnvalue (`SplineComponent.GetDistanceAlongSplineAtSplinePoint` _spline _stoppingpoint))
  (bind _returnvalue_2 (+ (`self.StoppingPoint`) 1))
  (bind (_output_requested _output_tower _output_approved _output_unhooked) (break `/Game/VTOL/VTOL_Struct` (`|GetArrayItem` (`self.TowerRequest`) _stoppingpoint_2)))
  (bind _returnvalue_3 (`SplineComponent.GetDistanceAlongSplineAtSplinePoint` _spline (+ _stoppingpoint 1)))
  (bind (_output_requested_2 _output_tower_2 _output_approved_2) (break `/Game/VTOL/VTOL_Struct` (`|GetArrayItem` (`self.TowerRequest`) _returnvalue_2)))
  (bind _returnvalue_4 (`KismetMathLibrary.Lerp` _returnvalue _returnvalue_3 (`self.Alpha`)))
  ;[1 1 1] Movement
  (if (`KismetMathLibrary.NearlyEqual_FloatFloat` (- _returnvalue_3 _returnvalue)) :!label _label
    (if (== (`self.StoppingPoint`) (- (`SplineComponent.GetNumberOfSplinePoints` _spline_2) 2)) :!label _label_2
      (`KismetSystemLibrary.Delay` 0.5)
      (`self.Land`)
      (else
        (if (not _output_unhooked)
          (`self.UnhookTower` _stoppingpoint_2))
        (if (not _output_requested_2)
          (`self.CreateRequest` _returnvalue_2))
        (if _output_approved_2
          (`/Engine/EditorBlueprintResources/StandardMacros.IncrementInt` (`self.StoppingPoint`)
            (:`  `
              (`self.Move`))))))
    (else
      (bind (_direction _alpha) (`Timeline|Drone Movement`)
        (:`Update`
          (set `self.Alpha` _alpha)
          (`self.K2_SetActorLocationAndRotation` (`SplineComponent.GetLocationAtDistanceAlongSpline` _spline_2 _returnvalue_4 "World") (`SplineComponent.GetRotationAtDistanceAlongSpline` _spline_2 _returnvalue_4 "World")))
        (:`Finished`
          (goto _label_2))))))

(event `Move`
  (bind _spline (`self.Spline`))
  (bind _stoppingpoint (`self.StoppingPoint`))
  (bind (_properties_height _properties_speed) (break `/Game/VTOL/VTOL_Properties` (`self.Properties`)))
  ;[1 1 1] Movement
  (`TimelineComponent.SetNewTime` (`self.Drone Movement`) 0.0)
  (`TimelineComponent.SetPlayRate` (`self.Drone Movement`) (/ 1.0 (/ (- (`SplineComponent.GetDistanceAlongSplineAtSplinePoint` _spline (+ _stoppingpoint 1)) (`SplineComponent.GetDistanceAlongSplineAtSplinePoint` _spline _stoppingpoint)) _properties_speed)))
  (`self.CreateRequest` (+ (`self.StoppingPoint`) 1))
  (goto _label))

(event `Land`
  (bind _stats_waitingtime (break `/Game/VTOL/VTOL_Stats` (`self.Stats`)))
  (bind (_properties_height _properties_speed _properties_destinationtower _properties_destinationpad) (break `/Game/VTOL/VTOL_Properties` (`self.Properties`)))
  ;[1 1 1] Land
  (bind _ashelipad_bp (cast `/Game/Objects/Helipad/Helipad_BP` _properties_destinationpad))
  (`SceneComponent.ToggleVisibility` (`self.Beam`) false)
  (bind (_direction _land) (`Timeline|Touchdown` :!via `PlayFromStart`)
    (:`Update`
      (bind _helipad (`/Game/Objects/Helipad/Helipad_BP.helipad` _ashelipad_bp))
      (bind (_returnvalue_x _returnvalue_y _returnvalue_z) (`KismetMathLibrary.BreakVector` (`SceneComponent.K2_GetComponentLocation` _helipad)))
      (`self.K2_SetActorLocationAndRotation` (`KismetMathLibrary.MakeVector` _returnvalue_x _returnvalue_y (`KismetMathLibrary.Lerp` (`self.Height`) (+ _returnvalue_z 50.0) _land)) (`KismetMathLibrary.RLerp` (`self.K2_GetActorRotation`) (`SceneComponent.K2_GetComponentRotation` _helipad) (/ _land 4.0) true)))
    (:`Finished`
      (`self.UnhookTower` (- (`KismetArrayLibrary.Array_Length` (`self.TowerRequest`)) 1))
      (`KismetSystemLibrary.Delay` 0.5)
      (`SceneComponent.SetVisibility` (`self.DefaultSceneRoot`) false true)
      (`SceneComponent.SetVisibility` (`self.Spline`) false true)
      (set `self.StatString` (`KismetStringLibrary.Concat_StrStr` (`KismetSystemLibrary.GetDisplayName` self) ":" " \\n" "Tower Waiting Times:" " \\n"))
      (for _array_element (`self.TowerRequest`)
        (bind _ascontrol_tower_bp2 (cast `/Game/Objects/ControlTower/ControlTowerBP2` (`.Tower_18_02CCCC744881AFC81EC09980D5DA025A` (break `/Game/VTOL/VTOL_Struct` _array_element))))
        (set `self.StatString` (`KismetStringLibrary.Concat_StrStr` (`self.StatString`) (`KismetSystemLibrary.GetDisplayName` _ascontrol_tower_bp2) ": " (`KismetStringLibrary.Conv_DoubleToString` (`BlueprintMapLibrary.Map_Find` _stats_waitingtime _ascontrol_tower_bp2)) " \\n")))
      (`PythonComponent.CallPythonComponentMethod` (`self.Python`) "SaveText" (`self.StatString`)))))

(fn `Approve`
  (params (Tower :type "/Game/Objects/ControlTower/ControlTowerBP2 Object Reference"))
  (locals (Index :type Integer))
  (bind _towerrequest (`self.TowerRequest`))
  (bind _time (`self.Time`))
  (bind _stats_waitingtime (break `/Game/VTOL/VTOL_Stats` (`self.Stats`)))
  (bind _output_get (set `local.Index` (`KismetArrayLibrary.Array_Find` _towerrequest (make `/Game/VTOL/VTOL_Struct` true Tower))))
  (setmembers `/Game/VTOL/VTOL_Struct` :`StructRef` (`|GetArrayItem` _towerrequest _output_get) :`Approved` true)
  (if (== (`local.Index`) 0)
    (`self.Liftoff`)
    (else
      (`self.Resume`)))
  (`BlueprintMapLibrary.Map_Add` _time "End" (`GameplayStatics.GetTimeSeconds`))
  (`BlueprintMapLibrary.Map_Add` _stats_waitingtime Tower (- (`BlueprintMapLibrary.Map_Find` _time "End") (`BlueprintMapLibrary.Map_Find` _time "Start"))))

(fn `UnhookTower`
  (params (Index :type Integer))
  (bind _towerrequest (`self.TowerRequest`))
  (bind (_output_requested _output_tower _output_approved) (break `/Game/VTOL/VTOL_Struct` (`|GetArrayItem` _towerrequest Index)))
  (`KismetArrayLibrary.Array_Set` _towerrequest Index (make `/Game/VTOL/VTOL_Struct` _output_requested _output_tower _output_approved true))
  (bind _ascontrol_tower_bp2 (cast `/Game/Objects/ControlTower/ControlTowerBP2` _output_tower))
  (`/Game/Objects/ControlTower/ControlTowerBP2.FinishedRequest` _ascontrol_tower_bp2 self "Moving"))

(fn `UserConstructionScript`)