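; Control tower actor that marks a circular airspace and shows its congestion by color.
; BeginPlay scales zone cylinders to Radius and randomizes helipad and building placement.
; Tick sphere-traces the zone, divides the hit count by 22, and tints the cylinder from green through yellow and orange to red.
; Requests go to a Python component; Approved and Denied only print, and older Blueprint redirect logic is disconnected.
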(event `self.ReceiveBeginPlay`
  (bind (_returnvalue_x _returnvalue_y _returnvalue_z) (`KismetMathLibrary.BreakVector` (`self.K2_GetActorLocation`)))
  (bind _returnvalue (/ (`self.Radius`) 50.0))
  ;[1 1 1] BeginPlay
  (set `self.Color` (`KismetMathLibrary.LinearColor_Green`))
  (`SceneComponent.SetWorldScale3D` (`self.Cylinder1`) (`KismetMathLibrary.MakeVector` _returnvalue _returnvalue 5.0))
  (`SceneComponent.SetWorldScale3D` (`self.Cylinder`) (`KismetMathLibrary.MakeVector` _returnvalue _returnvalue))
  (`SceneComponent.K2_SetWorldLocationAndRotation` (`self.helipad_mesh`) (`KismetMathLibrary.MakeVector` (+ _returnvalue_x (`KismetMathLibrary.RandomFloatInRange` 300.0 (- (`self.Radius`) 400.0))) _returnvalue_y _returnvalue_z) (`KismetMathLibrary.MakeRotator` 0.0 0.0 (`KismetMathLibrary.RandomFloatInRange` 0.0 360.0)) false false)
  (`SceneComponent.K2_SetWorldRotation` (`self.helipad_mesh`) (`KismetMathLibrary.MakeRotator` 0.0 0.0 (`KismetMathLibrary.RandomFloatInRange` 0.0 360.0)) false false)
  (`SceneComponent.K2_SetWorldRotation` (`self.Buildings`) (`KismetMathLibrary.MakeRotator` 0.0 0.0 (`KismetMathLibrary.RandomFloatInRange` 0.0 360.0)) false false)
  (`PrimitiveComponent.SetMaterial` (`self.Cube`) 0 (`|GetArrayItem` (`MeshComponent.GetMaterials` (`self.StaticMeshComponent`)))))

(event `Request`
  ;[1 1 1] Request
  (`PythonComponent.CallPythonComponentMethod` (`self.Python`) "Request" ""))

(event `Approved`
  ;[1 1 1] Request
  (`KismetSystemLibrary.PrintString` "--- Approved ---"))

(event `Denied`
  ;[1 1 1] Request
  (`KismetSystemLibrary.PrintString` "--- Denied ---"))

(event `self.ReceiveTick`
  (params (DeltaSeconds :type "Float (single-precision)"))
  (bind (_returnvalue_x _returnvalue_y) (`KismetMathLibrary.BreakVector` (`self.K2_GetActorLocation`)))
  ;[1 1 1] Event Tick
  (`GameplayStatics.GetAllActorsOfClass` "ControlTowerBP_C")
  (bind _outhits (`KismetSystemLibrary.SphereTraceMultiForObjects` :`Start` (`KismetMathLibrary.MakeVector` _returnvalue_x _returnvalue_y 1550.0) :`End` (`KismetMathLibrary.MakeVector` _returnvalue_x _returnvalue_y 1551.0) :`Radius` (+ (`self.Radius`) 100.0) :`ObjectTypes` (`self.ObjType`) :`DrawTime` 0.0))
  (bind _output_get (set `self.NumInRadius` (/ (`KismetArrayLibrary.Array_Length` _outhits) 22)))
  (switch `int` _output_get
    (:`Default`
      (set `self.Color` (`KismetMathLibrary.LinearColor_Red`) :!label _label))
    (:`0`
      (set `self.Color` (`KismetMathLibrary.LinearColor_Green`)))
    (:`1`
      (set `self.Color` (`KismetMathLibrary.LinearColor_Yellow`)))
    (:`2`
      (set `self.Color` (`KismetMathLibrary.MakeColor` 0.733333 0.263695 0.020763 0.0)))
    (:`3`
      (goto _label)))
  (`MeshComponent.SetVectorParameterValueOnMaterials` (`self.Cylinder`) "Param" (`KismetMathLibrary.Conv_LinearColorToVector` (`self.Color`))))

(fn `UserConstructionScript`)